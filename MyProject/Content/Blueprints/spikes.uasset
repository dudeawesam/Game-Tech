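; Spike hazard actor that destroys the first player's character whenever any actor begins overlapping it, with no damage step or check on the overlapping actor.
; On BeginPlay, each instance creates a Health_wg widget, adds it to the viewport and stores it in HealthBarReference.
; A separate HealthIsZero event clamps Health at zero but is not called here, and neither it nor the overlap updates the widget.
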(event `self.ReceiveActorBeginOverlap`
  (params (OtherActor :type "Actor Object Reference"))
  ;[1 1 1] Set health bar
  (`self.K2_DestroyActor` (`GameplayStatics.GetPlayerCharacter` 0)))

(event `self.ReceiveBeginPlay`
  (bind _returnvalue (`|CreateWidget` "/Game/Widget/Health_wg.Health_wg_C"))
  (`UserWidget.AddToViewport` _returnvalue 0)
  (set `self.health bar reference` _returnvalue))

(event `HealthIsZero`
  (if (<= (`self.Health`) 0.0)
    (set `self.Health` 0.0)))

(fn `UserConstructionScript`)