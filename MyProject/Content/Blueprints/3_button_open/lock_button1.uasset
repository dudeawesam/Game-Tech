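; Pressure switch actor that notifies a linked door when an actor steps on or off it, apparently part of a three-button door puzzle.
; Overlap begin and end call SwitchActivated and SwitchDeactivated on DoorToActivate and swap the switch mesh between on and off materials.
; The Switch_activate timeline plays and reverses to animate the switch's relative Z position.
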(event `self.ReceiveBeginPlay`)

(event `self.ReceiveActorBeginOverlap`
  (params (OtherActor :type "Actor Object Reference"))
  (`/Game/Blueprints/door_switch_BP.switch activated` (`self.door _to_activate`))
  (`PrimitiveComponent.SetMaterial` (`self.Switch`) 0 "/Game/switch_on_inst1.switch_on_inst1")
  (bind (_direction _switchpos) (`Timeline|switch_activate` :!label _label)
    (:`Update`
      (`SceneComponent.K2_SetRelativeLocation` (`self.Switch`) (`KismetMathLibrary.MakeVector` 0.0 0.0 _switchpos) false false))))

(event `self.ReceiveActorEndOverlap`
  (params (OtherActor :type "Actor Object Reference"))
  (`/Game/Blueprints/door_switch_BP.switch deactivated` (`self.door _to_activate`))
  (`PrimitiveComponent.SetMaterial` (`self.Switch`) 0 "/Game/switch_off_inst.switch_off_inst")
  (goto _label :!via `Reverse`))

(fn `UserConstructionScript`)