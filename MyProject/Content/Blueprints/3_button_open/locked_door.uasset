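; Locked door Blueprint that opens once three button locks have been released.
; Each Unlock_One call decrements and prints the remaining lock count, which Tick polls every frame, repeatedly triggering the unlock and a debug message while it is zero.
; The unlock event plays a timeline that slides the door mesh along Z.
; Leftover pressure switch events still update a counter, but their threshold checks do nothing.
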(event `self.ReceiveBeginPlay`
  (set `self.buttons_locked` 3))

(event `self.ReceiveTick`
  (params (DeltaSeconds :type "Float (single-precision)"))
  ;[1 1 1] Update Every Frame
  (if (== (`self.buttons_locked`) 0)
    (`self.Door_Unlocked`)
    (`KismetSystemLibrary.PrintString` "The door is unlocked")))

(event `Unlock_One`
  ;[1 1 1] Make Buttons Locked Go Down Then Print Value
  (set `self.buttons_locked` (- (`self.buttons_locked`) 1))
  (`KismetSystemLibrary.PrintString` (`KismetStringLibrary.Conv_IntToString` (`self.buttons_locked`))))

(event `Door_Unlocked`
  ;[1 1 1] Open Door
  (bind (_direction _open) (`Timeline|door opening`)
    (:`Update`
      (`SceneComponent.K2_SetRelativeLocation` (`self.Door`) (`KismetMathLibrary.MakeVector` 0.0 0.0 (* _open 205.0)) false false))))

(event `switch deactivated`
  ;[1 1 1] Code graveyard
  (`/Engine/EditorBlueprintResources/StandardMacros.DecrementInt` (`self.pressure_switches_active`)
    (:`  `
      (if (>= (`self.pressure_switches_active`) (`self.pressure_switches_needed`))
        _))))

(event `switch activated`
  ;[1 1 1] Code graveyard
  (`/Engine/EditorBlueprintResources/StandardMacros.IncrementInt` (`self.pressure_switches_active`)
    (:`  `
      (if (>= (`self.pressure_switches_active`) (`self.pressure_switches_needed`))
        _))))

(fn `UserConstructionScript`)