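; Laser hazard actor that fires a colored beam along its Arrow and hurts BP_ThirdPersonCharacter on contact with its Sphere.
; Each Tick a debug-drawn Camera-channel line trace sets the beam end point and shows the impact effect at hits.
; Distance snaps to the blocking hit and grows back over time up to a cap, so the beam extends gradually.
; Sphere overlap toggles the character's Hurting flag and starts DegenHealth on entry.
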(event `self.ReceiveBeginPlay`
  (`ActorComponent.SetActive` (`self.laser`) true false)
  (`ActorComponent.SetActive` (`self.laser impact`) true false)
  (`FXSystemComponent.SetColorParameter` (`self.laser impact`) "color" (struct :`R` 0.230708 :`G` 0.675112 :`B` 0.880208 :`A` 1.0))
  (`FXSystemComponent.SetColorParameter` (`self.laser`) "color" (struct :`R` 0.230708 :`G` 0.675112 :`B` 0.880208 :`A` 1.0)))

(event `self.ReceiveTick`
  (params (DeltaSeconds :type "Float (single-precision)"))
  (bind _returnvalue (`SceneComponent.K2_GetComponentLocation` (`self.Arrow`)))
  (bind _returnvalue_2 (+ _returnvalue (* (`SceneComponent.GetForwardVector` (`self.Arrow`)) (`self.distance`))))
  (`|ExecutionSequence`
    (:`then_0`
      (set `self.trace end` _returnvalue_2)
      (bind _outhit (`KismetSystemLibrary.LineTraceSingle` :`Start` _returnvalue :`End` _returnvalue_2 :`TraceChannel` "TraceTypeQuery2" :`DrawDebugType` "ForOneFrame"))
      (set `self.bHit` (`GameplayStatics.BreakHitResult` _outhit))
      (set `self.hit location` (`.Location` (`GameplayStatics.BreakHitResult` _outhit)))
      (`FXSystemComponent.SetVectorParameter` (`self.laser`) "laser end point" (select `bool` (`self.bHit`) :`false` (`self.trace end`) :`true` (`self.hit location`)))
      (`SceneComponent.SetVisibility` (`self.laser impact`) (`self.bHit`) false)
      (`SceneComponent.K2_SetWorldLocation` (`self.laser impact`) (`self.hit location`) false false)
      (if (`self.bHit`)
        (set `self.distance` (`KismetMathLibrary.VSize` (- (`self.hit location`) (`self.K2_GetActorLocation`))))))
    (:`then_1`
      (if (< (`self.distance`) 5000.0)
        (set `self.distance` (+ (`self.distance`) (* DeltaSeconds 2000.0)))))))

(event `self.Sphere.OnComponentBeginOverlap`
  (params (OverlappedComponent :type "PrimitiveComponent Object Reference") (OtherActor :type "Actor Object Reference") (OtherComp :type "PrimitiveComponent Object Reference") (OtherBodyIndex :type Integer) (bFromSweep :type Boolean) (SweepResult :type "HitResult Structure (by ref)"))
  (bind _asbp_third_person_character (cast `/Game/ThirdPerson/Blueprints/BP_ThirdPersonCharacter` OtherActor))
  (set `/Game/ThirdPerson/Blueprints/BP_ThirdPersonCharacter.Hurting?` true _asbp_third_person_character)
  (`/Game/ThirdPerson/Blueprints/BP_ThirdPersonCharacter.Degen Health` _asbp_third_person_character))

(event `self.Sphere.OnComponentEndOverlap`
  (params (OverlappedComponent :type "PrimitiveComponent Object Reference") (OtherActor :type "Actor Object Reference") (OtherComp :type "PrimitiveComponent Object Reference") (OtherBodyIndex :type Integer))
  (bind _asbp_third_person_character (cast `/Game/ThirdPerson/Blueprints/BP_ThirdPersonCharacter` OtherActor))
  (set `/Game/ThirdPerson/Blueprints/BP_ThirdPersonCharacter.Hurting?` false _asbp_third_person_character))

(fn `UserConstructionScript`)