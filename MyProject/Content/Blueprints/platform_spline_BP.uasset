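; Moving platform Blueprint that carries its static mesh along a referenced spline actor at a set speed.
; Each Tick adds speed-scaled delta time to a distance and applies the spline's local-space location there as the mesh's relative location, keeping its scale.
; When looping is enabled, the distance resets to zero after passing the spline's length.
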(event `self.ReceiveTick`
  (params (DeltaSeconds :type "Float (single-precision)"))
  (bind _returnvalue_location (`KismetMathLibrary.BreakTransform` (`SplineComponent.GetTransformAtDistanceAlongSpline` (`/Game/Blueprints/spline_path_BP.Spline` (`self.Spline to use`)) (`self.Distance`) "Local" false)))
  (set `self.Distance` (+ (* DeltaSeconds (`self.Speed`)) (`self.Distance`)))
  (`SceneComponent.K2_SetRelativeTransform` (`self.StaticMesh`) (`KismetMathLibrary.MakeTransform` _returnvalue_location (struct) (`SceneComponent.RelativeScale3D` (`self.StaticMesh`))) false false)
  (if (`self.is looped`)
    (if (> (`self.Distance`) (`SplineComponent.GetSplineLength` (`/Game/Blueprints/spline_path_BP.Spline` (`self.Spline to use`))))
      (set `self.Distance` 0.0))))

(fn `UserConstructionScript`)