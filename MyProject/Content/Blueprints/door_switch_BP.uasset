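; Door actor that opens when enough pressure switches are active at the same time.
; Custom events for switch activation and deactivation raise or lower an active count and compare it to the required number.
; The result plays or reverses the DoorOpening timeline, which slides the Door component vertically along its relative Z axis.
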(event `switch activated`
  (`/Engine/EditorBlueprintResources/StandardMacros.IncrementInt` (`self.pressure_switches_active`)
    (:`  `
      (if (>= (`self.pressure_switches_active`) (`self.pressure_switches_needed`))
        (bind (_direction _open) (`Timeline|door opening` :!label _label)
          (:`Update`
            (`SceneComponent.K2_SetRelativeLocation` (`self.Door`) (`KismetMathLibrary.MakeVector` 0.0 0.0 (* _open 205.0)) false false)))
        (else
          (goto _label :!via `Reverse`))))))

(event `switch deactivated`
  (`/Engine/EditorBlueprintResources/StandardMacros.DecrementInt` (`self.pressure_switches_active`)
    (:`  `
      (if (>= (`self.pressure_switches_active`) (`self.pressure_switches_needed`))
        (goto _label)
        (else
          (goto _label :!via `Reverse`))))))

(fn `UserConstructionScript`)