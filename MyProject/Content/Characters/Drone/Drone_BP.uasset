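; Enemy drone that wanders to random reachable points until it sees the player, then gives chase as a suicide attacker.
; PawnSensing triggers an AI move targeting the player controller; success damages the player and spawns an exploding drone, while failure resumes wandering.
; Player overlap with the Killbox triggers the player's damage reaction, scatters random health, coin or fuel pickups around a downward-traced ground point, and destroys the drone.
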(event `self.PawnSensing.OnSeePawn`
  (params (Pawn :type "Pawn Object Reference"))
  (cast `/Game/ThirdPerson/Blueprints/BP_ThirdPersonCharacter` Pawn)
  (set `self.isSeenPlayer?` true)
  (`self.Follow Player`))

(event `Follow Player`
  ;[1 1 1] Follow Player
  (if (`self.isSeenPlayer?`)
    (`|AIMoveTo` self (0.0 0.0 0.0) (`GameplayStatics.GetPlayerController` 0) 50.0
      (:`OnSuccess`
        (`self.K2_DestroyActor`)
        (bind _asbp_third_person_character (cast `/Game/ThirdPerson/Blueprints/BP_ThirdPersonCharacter` (`GameplayStatics.GetPlayerCharacter` 0)))
        (`GameplayStatics.ApplyDamage` _asbp_third_person_character 30.0)
        (`/Game/ThirdPerson/Blueprints/BP_ThirdPersonCharacter.Damage reaction` _asbp_third_person_character)
        (`|SpawnActorFromClass` "/Game/Blueprints/drone_exploding_BP.drone_exploding_BP_C" (`self.GetTransform`) "Undefined" "OverrideRootScale" null null))
      (:`OnFail`
        (set `self.isSeenPlayer?` false)))))

(event `self.ReceiveTick`
  (params (DeltaSeconds :type "Float (single-precision)"))
  (if (not (`self.isSeenPlayer?`))
    (`KismetSystemLibrary.Delay` 2.0)
    (`|AIMoveTo` self (`NavigationSystemV1.K2_GetRandomReachablePointInRadius` (`self.K2_GetActorLocation`) 500.0 null null) null)))

(event `self.Killbox.OnComponentBeginOverlap`
  (params (OverlappedComponent :type "PrimitiveComponent Object Reference") (OtherActor :type "Actor Object Reference") (OtherComp :type "PrimitiveComponent Object Reference") (OtherBodyIndex :type Integer) (bFromSweep :type Boolean) (SweepResult :type "HitResult Structure (by ref)"))
  (bind _asbp_third_person_character (cast `/Game/ThirdPerson/Blueprints/BP_ThirdPersonCharacter` OtherActor))
  (`/Game/ThirdPerson/Blueprints/BP_ThirdPersonCharacter.Damage reaction` _asbp_third_person_character)
  (for _ (range (+ (`KismetMathLibrary.RandomInteger` 2) 1))
    (`self.Drop Loot`))
  (`self.K2_DestroyActor`))

(event `Drop Loot`
  (bind _returnvalue (`self.K2_GetActorLocation`))
  ;[1 1 1] Drop Loot
  (bind _outhit (`KismetSystemLibrary.LineTraceSingle` _returnvalue (- _returnvalue (0.0 0.0 250.0)) "TraceTypeQuery1" false (`|MakeArray` (`GameplayStatics.GetPlayerCharacter` 0) :!type "Actor Object Reference")))
  (`|SpawnActorFromClass` (select `int` (`KismetMathLibrary.RandomInteger` 3) :`0` "/Game/Blueprints/Health_Pickup.Health_Pickup_C" :`1` "/Game/Blueprints/Coin_Pickup_BP.Coin_Pickup_BP_C" :`2` "/Game/Blueprints/Fuel_pickup_bp.Fuel_pickup_bp_C" :`3` null :!type "Actor Class Reference") (`KismetMathLibrary.MakeTransform` (`NavigationSystemV1.K2_GetRandomReachablePointInRadius` (`.Location` (`GameplayStatics.BreakHitResult` _outhit)) 75.0 null null) (`KismetMathLibrary.MakeRotator` 0.0 0.0 (`KismetMathLibrary.RandomFloatInRange` 0.0 350.0))) "Undefined" "OverrideRootScale" null null))

(fn `UserConstructionScript`)